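; BP_Crystal is a collectable crystal that flies into the player and vanishes when the player pawn overlaps it.
; A timeline's smooth alpha drives repeated lerps from the current location and scale toward the pawn's live position and a shrunken size, so the effect compounds each update.
; The timeline update also blacks out the point light and starts a short delay that destroys the actor.
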(event EventTick
  (params (DeltaSeconds :type Float%20%28single-precision%29)))

(event Collision|EventActorBeginOverlap
  (params (OtherActor :type Actor%20Object%20Reference))
  (if (== OtherActor (Game|Player|GetPlayerPawn 0))
    (bind _smoothlerpalpha (Timeline|TL_BlendAlpha Play)
      (:Update
        (Transformation|SetActorLocation (Math|Vector|Lerp(Vector) (Transformation|GetActorLocation) (Transformation|GetActorLocation (Game|Player|GetPlayerPawn 0)) _smoothlerpalpha) false false)
        (Transformation|SetActorScale3D (Math|Vector|Lerp(Vector) (Transformation|GetActorScale3D) (* (Transformation|GetActorScale3D) "0.100000,0.100000,0.100000") _smoothlerpalpha))
        (Rendering|Components|Light|SetLightColor :self (Variables|Default|GetPointLight))
        (Utilities|FlowControl|Delay 0.7)
        (Actor|DestroyActor)))))

(fn ConstructionScript)