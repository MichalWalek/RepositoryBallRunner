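; BP_WinVolume is a level-exit volume that lets the player finish once no BP_Crystal actors remain in the level.
; On player overlap it checks the crystal count, printing a Polish "not all crystals collected" message if any are left.
; Otherwise, after a short delay, it finds the current level's name in LevelList and opens the next entry, or quits the game on the last.
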(event Collision|EventActorBeginOverlap
  (params (OtherActor :type Actor%20Object%20Reference))
  (Utilities|IsPlayer OtherActor
    (:IsPlayer
      (bind _returnvalue (CallFunction|AllCrystals))
      (if _returnvalue
        (Utilities|FlowControl|Delay 1.0)
        (Utilities|IsLastIndex
          (:Return
            (CallFunction|Nexlevel)))
        (else
          (Development|PrintString "Nie zebrano wszystkich kryształów!" true true "(R=0.905758,G=0.053401,B=1.000000,A=1.000000)"))))))

(fn ConstructionScript)

(fn CheckAnyCrystals
  (Actor|GetAllActorsOfClass "/Game/Blueprints/Actors/Collectables/BP_Crystal.BP_Crystal_C"))

(fn AllCrystals
  (bind _outactors (Actor|GetAllActorsOfClass "/Game/Blueprints/Actors/Collectables/BP_Crystal.BP_Crystal_C"))
  (return (== (Utilities|Array|Length _outactors) 0)))

(fn CheckCurentIndeks
  (bind _returnvalue (Game|GetCurrentLevelName true))
  (return (Utilities|Array|FindItem (Variables|Default|GetLevelList) (Utilities|String|StringToName _returnvalue))))

(fn Nexlevel
  (Game|OpenLevel(byName) (Utilities|Array|Get(acopy) (Variables|Default|GetLevelList) (+ (CallFunction|CheckCurentIndeks) 1))))